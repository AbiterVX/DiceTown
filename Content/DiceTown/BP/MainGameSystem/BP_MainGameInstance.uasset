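; BP_MainGameInstance is the DiceTown game instance Blueprint, acting as a central manager for UI widgets.
; FunCreateUI adds a new widget to the viewport and records it in UserWidgetList, a map keyed by widget class.
; FunGetUI and FunRemoveUI look widgets up by class; removal detaches the widget but leaves its map entry.
; FunGetPlayerHeadImg ignores its path input and always returns one fixed avatar texture.
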(fn `Fun_CreateUI`
  (params (UserWidgetClass :type "UserWidget Class Reference") (OwningPlayer :type "PlayerController Object Reference"))
  (returns (UserWidget :type "UserWidget Object Reference"))
  (bind _returnvalue (`|CreateWidget` UserWidgetClass OwningPlayer))
  (`UserWidget.AddToViewport` _returnvalue 0)
  (`BlueprintMapLibrary.Map_Add` (`self.UserWidgetList`) (`GameplayStatics.GetObjectClass` _returnvalue) _returnvalue)
  (return _returnvalue))

(fn `Fun_GetPlayerHeadImg`
  (params (headImgPath :type String))
  (returns (HeadImg :type "Texture2D Object Reference"))
  (return "/Game/DiceTown/Resource/UI/HeadImg/T_HeadImg_2.T_HeadImg_2"))

(fn `Fun_GetUI`
  (params (UserWidgetClass :type "UserWidget Class Reference"))
  (returns (UI :type "UserWidget Object Reference"))
  (return (`BlueprintMapLibrary.Map_Find` (`self.UserWidgetList`) UserWidgetClass)))

(fn `Fun_RemoveUI`
  (params (UserWidgetClass :type "UserWidget Class Reference"))
  (bind (_value _returnvalue) (`BlueprintMapLibrary.Map_Find` (`self.UserWidgetList`) UserWidgetClass))
  (if _returnvalue
    (`Widget.RemoveFromParent` _value)))