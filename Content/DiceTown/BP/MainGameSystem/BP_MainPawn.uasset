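; BP_MainPawn is a main game pawn for DiceTown that handles camera zoom through its spring arm.
; Event_CameraZoom runs sequenced max and min checks that step or clamp the arm length, so an in-range zoom applies the step twice.
; ZoomMultiple stores the resulting length normalized between the arm limits.
; The forward and right movement events are empty stubs.
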(event `Event_CameraZoom`
  (params (Rate :type "Float (double-precision)"))
  (bind _armminlength (`self.ArmMinLength`))
  (bind _returnvalue (+ (`SpringArmComponent.TargetArmLength` (`self.SpringArm`)) (* (`self.ArmZoomStep`) Rate)))
  ;[1 1 1] Event:CameraZoom
  (`|ExecutionSequence`
    (:`then_0`
      (if (<= _returnvalue (`self.ArmMaxLength`))
        (set `SpringArmComponent.TargetArmLength` _returnvalue (`self.SpringArm`) :!label _label)
        (else
          (set `SpringArmComponent.TargetArmLength` (`self.ArmMaxLength`) (`self.SpringArm`)))))
    (:`then_1`
      (if (>= _returnvalue (`self.ArmMinLength`))
        (goto _label)
        (else
          (set `SpringArmComponent.TargetArmLength` (`self.ArmMinLength`) (`self.SpringArm`))))))
  ;[1 1 1] Comment
  (set `self.ZoomMultiple` (/ (- (`SpringArmComponent.TargetArmLength` (`self.SpringArm`)) _armminlength) (- (`self.ArmMaxLength`) _armminlength))))

(event `Event_MoveForward`
  (params (Rate :type "Float (double-precision)")))

(event `Event_MoveRight`
  (params (Rate :type "Float (double-precision)")))

(fn `UserConstructionScript`)