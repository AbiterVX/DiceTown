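; DiceTown's main game state Blueprint, providing current-player checks and a wait countdown.
; E_Init calls Init with Basic on the authority only.
; The player check converts a one-based player index to match the zero-based CurrentPlayerIndex.
; The countdown records a start time in server world time and derives the remaining time from WaitTimeMax, clamped at zero, so no ticking is needed.
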(event `E_Init`
  (`/Engine/EditorBlueprintResources/ActorMacros.Switch Has Authority`
    (:`Authority`
      (`self.init` "Basic"))))

(fn `F_GetRemainTime`
  (returns (RemainTime :type "Float (double-precision)"))
  (bind _returnvalue (- (+ (`self.StartTime`) (`self.WaitTimeMax`)) (`self.GetServerWorldTimeSeconds`)))
  (if (> _returnvalue 0.0)
    (return _returnvalue)
    (else
      (return 0.0))))

(fn `F_IfCurrentPlayer`
  (params (PLayerIndex :type Integer))
  (returns (ifCurrentPlayer :type Boolean))
  (return (== (`self.currentPlayerIndex`) (- PLayerIndex 1))))

(fn `F_SetStartTime`
  (set `self.StartTime` (`self.GetServerWorldTimeSeconds`)))

(fn `UserConstructionScript`)