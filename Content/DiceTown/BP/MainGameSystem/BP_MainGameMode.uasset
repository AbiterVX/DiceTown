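; Server game mode for DiceTown, a turn-based dice and city-building board game.
; It spawns a city per PlayerStart, then indexes and links joining players in ChoosePlayerStart.
; Dice panel choices roll for the current player and broadcast results; choice 3 advances game state, resolves buildings and refreshes UI.
; Buildings resolve as Red payments, then Blue and Green earnings; Special ones are only printed, and the win check is stubbed.
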(event `Event_PlayerAddLandScape`
  (params (PlaterIndex :type Integer) (LandScapeCount :type Integer))
  ;[1 1 1] Event:玩家增加地标
  ;;[1 1 1] 获取UI_Main界面的具体PlayerCityInfo的UI
  (bind _ui (`/Game/DiceTown/BP/MainGameSystem/BP_MainGameInstance.Fun_GetUI` (cast `/Game/DiceTown/BP/MainGameSystem/BP_MainGameInstance` (`GameplayStatics.GetGameInstance`) :!pure true) "/Game/DiceTown/BP/UI/UI_Main.UI_Main_C"))
  ;;[1 1 1] Landscape进度条平滑增加
  (bind (_direction _newtrack_0) (`Timeline|TimeLine_ProgressBar`)
    (:`Update`
      (bind (_materialinst _activedprocessbar) (`/Game/DiceTown/BP/UI/UI_PlayerCityInfo.Fun_GetProgressBar` (`BlueprintMapLibrary.Map_Find` (`/Game/DiceTown/BP/UI/UI_Main.PlayerCityInfoList` (cast `/Game/DiceTown/BP/UI/UI_Main` _ui :!pure true)) PlaterIndex) LandScapeCount))
      (`MaterialInstanceDynamic.SetScalarParameterValue` _materialinst "Percent" _newtrack_0)
      (`Image.SetBrushFromMaterial` _activedprocessbar _materialinst))))

(event `self.ReceiveBeginPlay`
  ;[1 1 1] BeginPlay
  (set `self.MainGameState` (cast `/Game/DiceTown/BP/MainGameSystem/BP_MainGameState` (`GameplayStatics.GetGameState`) :!pure true))
  (`/Game/DiceTown/BP/MainGameSystem/BP_MainGameState.E_Init` (`self.MainGameState`))
  (`/Engine/EditorBlueprintResources/ActorMacros.Switch Has Authority`
    (:`Authority`
      ;;[1 1 1] 创建PlayerCity
      (bind _outactors (`GameplayStatics.GetAllActorsOfClass` "/Script/Engine.PlayerStart"))
      (for _array_element _outactors
        (`BlueprintMapLibrary.Map_Add` (`self.PlayerStart`) (`KismetStringLibrary.Conv_StringToInt` (`KismetSystemLibrary.GetObjectName` _array_element)) _array_element)
        (bind _returnvalue (`|SpawnActorFromClass` "/Game/DiceTown/BP/DiceTown/BP_PlayerCity.BP_PlayerCity_C" (`self.GetTransform` (`self.GetAttachParentActor` _array_element)) "Undefined" "OverrideRootScale" null null))
        (`/Game/DiceTown/BP/DiceTown/BP_PlayerCity.E_Init` _returnvalue (`KismetStringLibrary.Conv_StringToInt` (`KismetSystemLibrary.GetObjectName` _array_element)))
        (`KismetArrayLibrary.Array_Add` (`self.PlayerCityList`) _returnvalue)))
    (:`Remote`)))

(event `Event_CountDown`
  (params (CountDownTime :type Integer))
  ;[1 1 1] Event:倒计时
  (set `self.CountDownTime` CountDownTime)
  (`KismetSystemLibrary.K2_SetTimer` null "Fun_CountDownPerSecond" 1.0 true))

(event `self.K2_PostLogin`
  (params (NewPlayer :type "PlayerController Object Reference"))
  ;[1 1 1] 玩家登录
)

(event `E_DicePanelChoice`
  (params (ChoiceIndex :type Integer))
  (bind _dicepoint (`/Game/DiceTown/BP/MainGameSystem/BP_MainGameState.DicePoint` (`self.MainGameState`)))
  ;[1 1 1] Event:骰子界面选择按钮
  ;;[1 1 1] 当前玩家投掷骰子
  (switch `int` ChoiceIndex
    (:`1`
      (bind _playercontroller (`self.F_GetCurrentPlayerController` :!label _label))
      (`self.F_GetDicePoint` ChoiceIndex _playercontroller))
    (:`2`
      (goto _label))
    (:`3`
      _)
    (:`4`
      _)
    (:`5`
      _))
  ;;[1 1 1] 所有玩家显示投掷结果
  (for _array_element (`self.playerList`)
    (`/Game/DiceTown/BP/MainGameSystem/BP_MainPlayerController.E_DicePanelCallBack` (cast `/Game/DiceTown/BP/MainGameSystem/BP_MainPlayerController` _array_element :!pure true) ChoiceIndex _dicepoint)
    ;;[1 1 1] 触发骰子效果
    (if (== ChoiceIndex 3)
      ;;;[1 1 1] 下一阶段
      (`MainGameState.startNextState` (`self.MainGameState`))
      (`/Game/DiceTown/BP/DiceTown/BPFL.F_PrintDicePoint` _dicepoint)
      (`self.F_TriggerBuilding`)
      ;;[1 1 1] 刷新UI
      (`self.F_RefreshPlayerUI`))))

(fn `ChoosePlayerStart`
  (params (Player :type "Controller Object Reference"))
  (returns (ReturnValue :type "Actor Object Reference"))
  (bind _asbp_main_player_controller (cast `/Game/DiceTown/BP/MainGameSystem/BP_MainPlayerController` Player :!pure true))
  (bind _playerindex (`/Game/DiceTown/BP/MainGameSystem/BP_MainPlayerController.PlayerIndex` _asbp_main_player_controller))
  (`/Engine/EditorBlueprintResources/ActorMacros.Switch Has Authority`
    (:`Authority`
      ;[1 1 1] 添加Player
      (bind _output_get (set `self.PlayerCount` (+ (`self.PlayerCount`) 1)))
      (bind _output_get_2 (set `/Game/DiceTown/BP/MainGameSystem/BP_MainPlayerController.PlayerIndex` _output_get _asbp_main_player_controller))
      (`KismetSystemLibrary.PrintString` (`KismetStringLibrary.Concat_StrStr` "PLayer:" (`KismetStringLibrary.Conv_IntToString` _output_get_2)) true true (struct :`G` 0.66 :`B` 1.0 :`A` 1.0) 100.0)
      (bind _returnplayercity (`self.F_GetPLayerCity` _playerindex))
      (`/Game/DiceTown/BP/MainGameSystem/BP_MainPlayerController.E_Init` _asbp_main_player_controller _playerindex _returnplayercity)
      (`MainPlayerState.setPlayerInfo` (cast `MainPlayerState` (`Controller.PlayerState` _asbp_main_player_controller) :!pure true) _playerindex _playerindex (`KismetStringLibrary.Concat_StrStr` "Name:" (`KismetStringLibrary.Conv_IntToString` _playerindex)) _returnplayercity)
      (`self.addPlayer` _asbp_main_player_controller))
    (:`Remote`
      _))
  (return (`BlueprintMapLibrary.Map_Find` (`self.PlayerStart`) (`/Game/DiceTown/BP/MainGameSystem/BP_MainPlayerController.PlayerIndex` _asbp_main_player_controller))))

(fn `F_GetCurrentPlayerController`
  (returns (PlayerController :type "/Game/DiceTown/BP/MainGameSystem/BP_MainPlayerController Object Reference"))
  (for _array_element (`self.playerList`)
    (bind _asbp_main_player_controller (cast `/Game/DiceTown/BP/MainGameSystem/BP_MainPlayerController` _array_element :!pure true))
    (if (== (`/Game/DiceTown/BP/MainGameSystem/BP_MainPlayerController.PlayerIndex` _asbp_main_player_controller) (+ (`MainGameState.currentPlayerIndex` (`self.MainGameState`)) 1))
      (return _asbp_main_player_controller)))
  (return null))

(fn `F_GetDicePoint`
  (params (DiceCount :type Integer) (CurrentPlayerController :type "/Game/DiceTown/BP/MainGameSystem/BP_MainPlayerController Object Reference"))
  (bind _ifcurrentplayer (`/Game/DiceTown/BP/MainGameSystem/BP_MainGameState.F_IfCurrentPlayer` (`self.MainGameState`) (`/Game/DiceTown/BP/MainGameSystem/BP_MainPlayerController.PlayerIndex` CurrentPlayerController)))
  (if _ifcurrentplayer
    (bind _returnvalue (`self.getDicePoint` DiceCount))
    (set `/Game/DiceTown/BP/MainGameSystem/BP_MainGameState.DicePoint` _returnvalue (`self.MainGameState`))
    (return)
    (else
      (return))))

(fn `F_GetPLayerCity`
  (params (PlayerIndex :type Integer))
  (returns (ReturnPlayerCity :type "/Game/DiceTown/BP/DiceTown/BP_PlayerCity Object Reference"))
  (locals (AvaliablePlayerCity :type "/Game/DiceTown/BP/DiceTown/BP_PlayerCity Object Reference"))
  (for _array_element (`self.PlayerCityList`)
    (if (== (`PlayerCity.playerIndex` _array_element) PlayerIndex)
      (return _array_element)))
  (return null))

(fn `F_RefreshPlayerUI`
  (for _array_element (`self.playerList`)
    (`/Game/DiceTown/BP/MainGameSystem/BP_MainPlayerController.E_RefreshUI` (cast `/Game/DiceTown/BP/MainGameSystem/BP_MainPlayerController` _array_element :!pure true))))

(fn `F_TriggerBuilding`
  (locals (PayMessages :type "Array of StructMessage Structure") (CurrentPC :type "/Game/DiceTown/BP/MainGameSystem/BP_MainPlayerController Object Reference"))
  (bind _currentpc (`local.CurrentPC`))
  (bind _currentpc_2 (`local.CurrentPC`))
  (bind _playercity (`/Game/DiceTown/BP/MainGameSystem/BP_MainPlayerController.PlayerCity` _currentpc_2))
  (bind _playercontroller (`self.F_GetCurrentPlayerController`))
  (set `local.CurrentPC` _playercontroller)
  ;[1 1 1] 1.激活其他玩家【Red类型】建筑
  (for (_array_element _array_index) (`self.playerList`)
    (if (!= _array_index (- (`/Game/DiceTown/BP/MainGameSystem/BP_MainPlayerController.PlayerIndex` (`local.CurrentPC`)) 1))
      (bind _asbp_main_player_controller (cast `/Game/DiceTown/BP/MainGameSystem/BP_MainPlayerController` _array_element :!pure true))
      (bind _triggermessages (`/Game/DiceTown/BP/MainGameSystem/BP_MainPlayerController.F_GetTriggerMessage` _asbp_main_player_controller "Other" (`/Game/DiceTown/BP/MainGameSystem/BP_MainPlayerController.PlayerCity` _asbp_main_player_controller)))
      (`KismetArrayLibrary.Array_Append` (`local.PayMessages`) _triggermessages)))
  ;[1 1 1] 2.其他玩家获取收益&当前玩家支付所需费用
  (bind _returnvalue (`PlayerCity.triggerPay` (`/Game/DiceTown/BP/MainGameSystem/BP_MainPlayerController.PlayerCity` (`local.CurrentPC`)) (`local.PayMessages`)))
  (for _array_element_2 (`self.PlayerList`)
    (bind _playercity_2 (`/Game/DiceTown/BP/MainGameSystem/BP_MainPlayerController.PlayerCity` (cast `/Game/DiceTown/BP/MainGameSystem/BP_MainPlayerController` _array_element_2 :!pure true)))
    (bind _playerindex (`PlayerCity.playerIndex` _playercity_2))
    (if (!= _playerindex (`/Game/DiceTown/BP/MainGameSystem/BP_MainPlayerController.PlayerIndex` (`local.CurrentPC`)))
      (`PlayerCity.getPayEarn` _playercity_2 (`|GetArrayItem` _returnvalue (- _playerindex 1)))))
  ;[1 1 1] 3.激活所有玩家【Blue类型】建筑 & 获取收益
  (for _array_element_3 (`self.PlayerList`)
    (bind _asbp_main_player_controller_2 (cast `/Game/DiceTown/BP/MainGameSystem/BP_MainPlayerController` _array_element_3 :!pure true))
    (bind _playercity_3 (`/Game/DiceTown/BP/MainGameSystem/BP_MainPlayerController.PlayerCity` _asbp_main_player_controller_2))
    (bind _triggermessages_2 (`/Game/DiceTown/BP/MainGameSystem/BP_MainPlayerController.F_GetTriggerMessage` _asbp_main_player_controller_2 "All" _playercity_3))
    (bind _returnvalue_2 (`PlayerCity.triggerNormalEarn` _playercity_3 _triggermessages_2))
    (`PlayerCity.getPayEarn` _playercity_3 (`|GetArrayItem` _returnvalue_2 (- (`PlayerCity.playerIndex` _playercity_3) 1))))
  ;[1 1 1] 4.激活当前玩家【Green类型】建筑 & 获取收益
  (bind _triggermessages_3 (`/Game/DiceTown/BP/MainGameSystem/BP_MainPlayerController.F_GetTriggerMessage` _currentpc_2 "Self" _playercity))
  (bind _returnvalue_3 (`PlayerCity.triggerNormalEarn` _playercity _triggermessages_3))
  (`PlayerCity.getPayEarn` _playercity (`|GetArrayItem` _returnvalue_3 (- (`PlayerCity.playerIndex` _playercity) 1)))
  ;[1 1 1] 5.激活当前玩家【Special类型】建筑 & 获取收益/触发效果
  (bind _triggermessages_4 (`/Game/DiceTown/BP/MainGameSystem/BP_MainPlayerController.F_GetTriggerMessage` _currentpc "Special" (`/Game/DiceTown/BP/MainGameSystem/BP_MainPlayerController.PlayerCity` _currentpc)))
  (`/Game/DiceTown/BP/DiceTown/BPFL.F_PrintTriggerMessages` _triggermessages_4))

(fn `Fun_CountDownPerSecond`
  (bind _returnvalue (- (`self.CountDownTime`) 1))
  (if (<= _returnvalue 0)
    (set `self.CountDownTime` 0)
    (else
      (set `self.CountDownTime` _returnvalue))))

(fn `Fun_IfWin`
  (returns (Index :type Integer)))

(fn `Fun_InitJson_DiceSkill`
  (params (SkillIndex :type Integer) (DicePoint :type "Array of Integer"))
  (returns (JsonParam :type "StructJsonObject Structure"))
  (locals (DiceSkillType :type "EDiceSkillType Enum"))
  (switch `int` SkillIndex
    (:`3`
      (set `local.DiceSkillType` "None"))
    (:`4`
      (set `local.DiceSkillType` "ReRoll"))
    (:`5`
      (set `local.DiceSkillType` "AddTwo")))
  (bind _returnvalue (`BPLibraryUtils.makeJson`))
  (bind _returnvalue_2 (`BPLibraryUtils.setNumberValue` _returnvalue "SkillIndex" (`KismetMathLibrary.Conv_ByteToInt` (`local.DiceSkillType`))))
  (bind _returnvalue_3 (`BPLibraryUtils.setNumberArrayValue` _returnvalue_2 "DicePoint" DicePoint))
  (return _returnvalue_3))

(fn `Fun_InitJson_GetDicePoint`
  (params (DicePoint :type "Array of Integer"))
  (returns (ReturnValue :type "StructJsonObject Structure")))

(fn `UserConstructionScript`)