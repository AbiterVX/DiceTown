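; Player controller for DiceTown, a multiplayer dice-driven city-building game, bridging the local UI, camera pawn and server game mode.
; Local players get the main UI, a delayed refresh of building and player panels, and lockable drag and zoom camera controls.
; Dice choices go to the server, with results returned to the owning client's UI.
; On authority, FTriggerBuilding resolves building payouts in Red, Blue, Green, Special order, though Special only prints messages.
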(event `self.ReceiveBeginPlay`
  ;[1 1 1] Event:BeginPlay
  ;;[1 1 1] GameState
  (set `self.MainGameState` (cast `/Game/DiceTown/BP/MainGameSystem/BP_MainGameState` (`GameplayStatics.GetGameState`) :!pure true))
  ;;[1 1 1] 设置GameInstance
  (set `self.MainGameInstance` (cast `/Game/DiceTown/BP/MainGameSystem/BP_MainGameInstance` (`GameplayStatics.GetGameInstance`) :!pure true))
  ;;[1 1 1] Pawn
  (set `self.MainPawn` (cast `/Game/DiceTown/BP/MainGameSystem/BP_MainPawn` (`self.K2_GetPawn`) :!pure true))
  ;;[1 1 1] 显示:UI, 设置鼠标
  (if (`self.IsLocalController`)
    (bind _userwidget (`/Game/DiceTown/BP/MainGameSystem/BP_MainGameInstance.Fun_CreateUI` (`self.MainGameInstance`) "/Game/DiceTown/BP/UI/UI_Main.UI_Main_C" self))
    (set `self.UIMain` (cast `/Game/DiceTown/BP/UI/UI_Main` _userwidget :!pure true))
    (set `self.bShowMouseCursor` true)
    ;;[1 1 1] 刷新UI
    (`KismetSystemLibrary.K2_SetTimer` null "E_RefreshUI" 2.0)))

(event `self.ReceiveTick`
  (params (DeltaSeconds :type "Float (single-precision)"))
  (bind (_sizex _sizey) (`self.GetViewportSize`))
  (bind (_locationx _locationy _returnvalue) (`self.GetMousePosition`))
  (bind (_mouseanchorpoint_x _mouseanchorpoint_y) (`KismetMathLibrary.BreakVector2D` (`self.MouseAnchorPoint`)))
  (bind _movestep (`self.MoveStep`))
  ;[1 1 1] EventTick:
  (if (and (`self.IsLocalController`) (`KismetSystemLibrary.IsValid` (`self.MainPawn`)))
    ;;[1 1 1] 鼠标拖拽
    (`self.Macro_IfDragUnlocked`
      (:`true`
        (if (and (`self.HasPressed`) _returnvalue)
          (`PawnMovementComponent.AddInputVector` (`/Game/DiceTown/BP/MainGameSystem/BP_MainPawn.FloatingPawnMovement` (`self.MainPawn`)) (* (`KismetMathLibrary.MakeVector` (* (* (/ (- _locationy _mouseanchorpoint_y) (`KismetMathLibrary.Conv_IntToDouble` _sizey)) _movestep) -1.0) (* (* (/ (- _locationx _mouseanchorpoint_x) (`KismetMathLibrary.Conv_IntToDouble` _sizex)) _movestep) 1.0)) (`/Game/DiceTown/BP/MainGameSystem/BP_MainPawn.ZoomMultiple` (`self.MainPawn`))) false)
          (set `self.MouseAnchorPoint` (`KismetMathLibrary.MakeVector2D` _locationx _locationy)))))))

(event `E_RefreshUI`
  ;[1 1 1] Event:刷新UI
  (`self.E_RefreshUIBuildingList`)
  (for _array_element (`GameStateBase.PlayerArray` (`self.MainGameState`))
    (bind _asbp_main_player_state (cast `/Game/DiceTown/BP/MainGameSystem/BP_MainPlayerState` _array_element :!pure true))
    (bind _playerindex (`MainPlayerState.playerIndex` _asbp_main_player_state))
    (bind _returnplayercity (`/Game/DiceTown/BP/MainGameSystem/BP_MainGameMode.F_GetPLayerCity` (cast `/Game/DiceTown/BP/MainGameSystem/BP_MainGameMode` (`GameplayStatics.GetGameMode`) :!pure true) _playerindex))
    (`self.E_RefreshPlayerUI` (`MainPlayerState.playerInfo` _asbp_main_player_state) _playerindex (`PlayerCity.money` _returnplayercity) (`KismetArrayLibrary.Array_Length` (`PlayerCity.buildingList` _returnplayercity)) (`KismetArrayLibrary.Array_Length` (`PlayerCity.landmarkList` _returnplayercity)))))

(event `E_Init`
  (params (PlayerIndex :type Integer) (PlayerCity :type "/Game/DiceTown/BP/DiceTown/BP_PlayerCity Object Reference"))
  ;[1 1 1] Event(Mulitcast):Init
  ;;[1 1 1] Index
  (set `self.PlayerIndex` PlayerIndex)
  ;;[1 1 1] City
  (set `self.PlayerCity` PlayerCity))

(event `E_SetDragLocked`
  (params (dragLocked :type Boolean))
  ;[1 1 1] Event:设置拖拽锁定
  (set `self.DragLocked` dragLocked))

(event `InputAction|CameraZoomIn`
  (params (Key :type "Key Structure"))
  ;[1 1 1] Input:摄像头距离缩放
  (:`Pressed`
    (`self.Macro_IfDragUnlocked`
      (:`true`
        (`/Game/DiceTown/BP/MainGameSystem/BP_MainPawn.Event_CameraZoom` (`self.MainPawn`) -1.0)))))

(event `InputAction|MainClick`
  (params (Key :type "Key Structure"))
  (bind (_locationx _locationy) (`self.GetMousePosition`))
  ;[1 1 1] Input: MainClick
  (:`Pressed`
    ;;[1 1 1] 屏幕鼠标拖拽
    (set `self.MouseAnchorPoint` (`KismetMathLibrary.MakeVector2D` _locationx _locationy))
    (set `self.HasPressed` true))
  (:`Released`
    (set `self.HasPressed` false)))

(event `InputAction|CameraZoomOut`
  (params (Key :type "Key Structure"))
  ;[1 1 1] Input:摄像头距离缩放
  (:`Pressed`
    (`self.Macro_IfDragUnlocked`
      (:`true`
        (`/Game/DiceTown/BP/MainGameSystem/BP_MainPawn.Event_CameraZoom` (`self.MainPawn`) 1.0)))))

(event `E_RefreshUIBuildingList`
  ;[1 1 1] EventUI(Run on Owning Client):刷新建筑列表
  (if (`self.IsLocalController`)
    (`/Game/DiceTown/BP/UI/UI_Main.E_RefreshBuildingInfoList` (`self.UIMain`) (`/Game/DiceTown/BP/DiceTown/BP_PlayerCity.currentUIBuildingList` (`self.PlayerCity`)))))

(event `E_RefreshPlayerUI`
  (params (`PlayerInfo ` :type "StructPlayer Structure (by ref)") (PlayerIndex :type Integer) (MoneyCount :type Integer) (BuildingCount :type Integer) (LandmarkCount :type Integer))
  (bind (_userid _password _phonenumber _headimgpath _username) (break `StructPlayer` `PlayerInfo `))
  (bind _maingameinstance (`self.MainGameInstance`))
  ;[1 1 1] Event(Run on Owning Client):添加玩家UI
  (if (`self.IsLocalController`)
    (if (not (== _userid -1))
      (bind _ui (`/Game/DiceTown/BP/MainGameSystem/BP_MainGameInstance.Fun_GetUI` _maingameinstance "/Game/DiceTown/BP/UI/UI_Main.UI_Main_C"))
      (bind _headimg (`/Game/DiceTown/BP/MainGameSystem/BP_MainGameInstance.Fun_GetPlayerHeadImg` _maingameinstance _headimgpath))
      (`/Game/DiceTown/BP/UI/UI_Main.E_RefreshPlayer` (cast `/Game/DiceTown/BP/UI/UI_Main` _ui :!pure true) _username _headimg PlayerIndex MoneyCount BuildingCount LandmarkCount))))

(event `InputAxis|CameraMoveForward`
  (params (AxisValue :type "Float (single-precision)"))
  (bind _mainpawn (`self.MainPawn`))
  ;[1 1 1] Input:WSAD控制镜头移动（测试）
  (if (`KismetSystemLibrary.IsValid` _mainpawn)
    (`PawnMovementComponent.AddInputVector` (`/Game/DiceTown/BP/MainGameSystem/BP_MainPawn.FloatingPawnMovement` _mainpawn) (`KismetMathLibrary.MakeVector` (* AxisValue -10.0)) false)))

(event `InputAction|TestBtn_1`
  (params (Key :type "Key Structure"))
  (bind _uimain (`self.UIMain`))
  ;[1 1 1] Input:测试按钮 E
  (:`Pressed`
    (`/Engine/EditorBlueprintResources/StandardMacros.FlipFlop`
      (:`A`
        (`/Game/DiceTown/BP/UI/UI_Main.E_ShowRollDicePanel` _uimain true))
      (:`B`
        (`/Game/DiceTown/BP/UI/UI_Main.E_ShowRollDicePanel` _uimain false)))))

(event `E_DicePanelChoice`
  (params (ChoiceIndex :type Integer :default -1))
  ;[1 1 1] Event(Run on Server):骰子界面选择按钮
  (`/Game/DiceTown/BP/MainGameSystem/BP_MainGameMode.E_DicePanelChoice` (cast `/Game/DiceTown/BP/MainGameSystem/BP_MainGameMode` (`GameplayStatics.GetGameMode`) :!pure true) ChoiceIndex))

(event `InputAxis|CameraMoveRight`
  (params (AxisValue :type "Float (single-precision)"))
  (bind _mainpawn (`self.MainPawn`))
  ;[1 1 1] Input:WSAD控制镜头移动（测试）
  (if (`KismetSystemLibrary.IsValid` _mainpawn)
    (`PawnMovementComponent.AddInputVector` (`/Game/DiceTown/BP/MainGameSystem/BP_MainPawn.FloatingPawnMovement` _mainpawn) (`KismetMathLibrary.MakeVector` 0.0 (* AxisValue -10.0)) false)))

(event `E_ShowTriggerBuildingPanel`
  (params (IsShow :type Boolean))
  (`/Game/DiceTown/BP/UI/UI_Main.E_ShowTriggerBuildingPanel` (`self.UIMain`) IsShow))

(event `InputAction|TestBtn_2`
  (params (Key :type "Key Structure"))
  ;[1 1 1] Input:测试按钮 F
  (:`Pressed`
    (bind _isa (`/Engine/EditorBlueprintResources/StandardMacros.FlipFlop`)
      (:`A`
        _)
      (:`B`
        _))
    (`/Game/DiceTown/BP/UI/UI_Main.E_ShowTriggerBuildingPanel` (`self.UIMain`) _isa)))

(event `E_DicePanelCallBack`
  (params (ChoiceIndex :type Integer) (DicePoint :type "Array of Integer"))
  (bind _uimain (`self.UIMain`))
  ;[1 1 1] Event(Run on Owning Client):骰子界面回调
  (`/Engine/EditorBlueprintResources/ActorMacros.Switch Has Authority`
    (:`Remote`
      (bind _ifcurrentplayer (`/Game/DiceTown/BP/MainGameSystem/BP_MainGameState.F_IfCurrentPlayer` (`self.MainGameState`) (`self.PlayerIndex`)))
      (switch `int` ChoiceIndex
        (:`1`
          (`/Game/DiceTown/BP/UI/UI_Main.E_RollDiceCallback` _uimain DicePoint _ifcurrentplayer :!label _label))
        (:`2`
          (goto _label))
        (:`3`
          (`/Game/DiceTown/BP/UI/UI_Main.E_ShowRollDicePanel` _uimain false))
        (:`4`
          (if _ifcurrentplayer
            (`/Game/DiceTown/BP/UI/UI_Main.E_ShowRollDicePanel` _uimain true)))))))

(event `Event_ShopPanelChoice`
  (params (ChoiceIndex :type Integer :default -1) (BuildingIndex :type Integer))
  ;[1 1 1] Event:商店界面选择按钮回调
  (switch `int` ChoiceIndex
    (:`2`
      (`self.E_ShowShopPanel` false))))

(event `InputAction|TestBtn_3`
  (params (Key :type "Key Structure"))
  ;[1 1 1] Input:测试按钮 G
  (:`Pressed`
    (if true
      _)))

(event `E_ShowShopPanel`
  (params (isShow :type Boolean))
  ;[1 1 1] 显示商店界面
  (`/Game/DiceTown/BP/UI/UI_Main.Event_ShowShopPanel` (`self.UIMain`) isShow))

(event `E_ShowDicePanel`
  (params (isShow :type Boolean))
  ;[1 1 1] 显示骰子界面
  (`/Game/DiceTown/BP/UI/UI_Main.E_ShowRollDicePanel` (`self.UIMain`) isShow))

(fn `F_GetTriggerMessage`
  (params (_BuildingType :type "EBuildingType Enum" :default "Self") (PlayerCity :type "PlayerCity Object Reference"))
  (returns (TriggerMessages :type "Array of StructMessage Structure"))
  (bind _maingamestate (`self.MainGameState`))
  (bind _returnvalue (`PlayerCity.getTriggerMessages` PlayerCity (`/Game/DiceTown/BP/MainGameSystem/BP_MainGameState.DicePoint` _maingamestate) (`/Game/DiceTown/BP/MainGameSystem/BP_MainGameState.DiceSkill` _maingamestate) _BuildingType))
  (return _returnvalue))

(fn `F_IsMyBuildState`
  (returns (IsMyBuildState :type Boolean))
  (bind _maingamestate (`self.MainGameState`))
  (bind _ifcurrentplayer (`/Game/DiceTown/BP/MainGameSystem/BP_MainGameState.F_IfCurrentPlayer` _maingamestate (`self.PlayerIndex`)))
  (bind _returnvalue (`MainGameState.isBuildState` _maingamestate))
  (return (and _returnvalue _ifcurrentplayer)))

(fn `F_IsMyDiceState`
  (returns (IsMyDiceState :type Boolean))
  (bind _maingamestate (`self.MainGameState`))
  (bind _ifcurrentplayer (`/Game/DiceTown/BP/MainGameSystem/BP_MainGameState.F_IfCurrentPlayer` _maingamestate (`self.PlayerIndex`)))
  (bind _returnvalue (`MainGameState.isDiceState` _maingamestate))
  (return (and _returnvalue _ifcurrentplayer)))

(fn `F_TriggerBuilding`
  (locals (PayMessages :type "Array of StructMessage Structure") (PlayerList :type "Array of MainPlayerController Object Reference"))
  (bind _playercity (`self.PlayerCity`))
  (`/Engine/EditorBlueprintResources/ActorMacros.Switch Has Authority`
    (:`Authority`
      ;[1 1 1] PlayerList
      (set `local.PlayerList` (`MainGameMode.playerList` (cast `/Game/DiceTown/BP/MainGameSystem/BP_MainGameMode` (`GameplayStatics.GetGameMode`) :!pure true)))
      ;[1 1 1] 1.激活其他玩家【Red类型】建筑
      (for (_array_element _array_index) (`local.PlayerList`)
        (if (!= _array_index (- (`self.PlayerIndex`) 1))
          (bind _asbp_main_player_controller (cast `/Game/DiceTown/BP/MainGameSystem/BP_MainPlayerController` _array_element :!pure true))
          (bind _triggermessages (`self.F_GetTriggerMessage` _asbp_main_player_controller "Other" (`/Game/DiceTown/BP/MainGameSystem/BP_MainPlayerController.PlayerCity` _asbp_main_player_controller)))
          (`KismetArrayLibrary.Array_Append` (`local.PayMessages`) _triggermessages)))
      ;[1 1 1] 2.其他玩家获取收益&当前玩家支付所需费用
      (bind _returnvalue (`PlayerCity.triggerPay` (`self.PlayerCity`) (`local.PayMessages`)))
      (for _array_element_2 (`local.PlayerList`)
        (bind _playercity_2 (`/Game/DiceTown/BP/MainGameSystem/BP_MainPlayerController.PlayerCity` (cast `/Game/DiceTown/BP/MainGameSystem/BP_MainPlayerController` _array_element_2 :!pure true)))
        (bind _playerindex (`PlayerCity.playerIndex` _playercity_2))
        (if (!= _playerindex (`self.PlayerIndex`))
          (`PlayerCity.getPayEarn` _playercity_2 (`|GetArrayItem` _returnvalue (- _playerindex 1)))))
      ;[1 1 1] 3.激活所有玩家【Blue类型】建筑 & 获取收益
      (for _array_element_3 (`local.PlayerList`)
        (bind _asbp_main_player_controller_2 (cast `/Game/DiceTown/BP/MainGameSystem/BP_MainPlayerController` _array_element_3 :!pure true))
        (bind _playercity_3 (`/Game/DiceTown/BP/MainGameSystem/BP_MainPlayerController.PlayerCity` _asbp_main_player_controller_2))
        (bind _triggermessages_2 (`self.F_GetTriggerMessage` _asbp_main_player_controller_2 "All" _playercity_3))
        (bind _returnvalue_2 (`PlayerCity.triggerNormalEarn` _playercity_3 _triggermessages_2))
        (`PlayerCity.getPayEarn` _playercity_3 (`|GetArrayItem` _returnvalue_2 (- (`PlayerCity.playerIndex` _playercity_3) 1))))
      ;[1 1 1] 4.激活当前玩家【Green类型】建筑 & 获取收益
      (bind _triggermessages_3 (`self.F_GetTriggerMessage` "Self" _playercity))
      (bind _returnvalue_3 (`PlayerCity.triggerNormalEarn` _playercity _triggermessages_3))
      (`PlayerCity.getPayEarn` _playercity (`|GetArrayItem` _returnvalue_3 (- (`PlayerCity.playerIndex` _playercity) 1)))
      ;[1 1 1] 5.激活当前玩家【Special类型】建筑 & 获取收益/触发效果
      (bind _triggermessages_4 (`self.F_GetTriggerMessage` "Special" (`self.PlayerCity`)))
      (`/Game/DiceTown/BP/DiceTown/BPFL.F_PrintTriggerMessages` _triggermessages_4))))

(fn `Fun_InitJson_DiceSkill`
  (params (DicePoint :type "Array of Integer") (SkillIndex :type Integer))
  (returns (JsonObject :type "StructJsonObject Structure"))
  (bind _returnvalue (`BPLibraryUtils.makeJson`))
  (bind _returnvalue_2 (`BPLibraryUtils.setNumberArrayValue` _returnvalue "DicePoint" DicePoint))
  (bind _returnvalue_3 (`BPLibraryUtils.setNumberValue` _returnvalue_2 "SkillIndex" SkillIndex))
  (return _returnvalue_3))

(fn `Fun_InitJson_GetDicePoint`
  (params (DiceNum :type Integer))
  (returns (JsonObject :type "StructJsonObject Structure"))
  (bind _returnvalue (`BPLibraryUtils.makeJson`))
  (bind _returnvalue_2 (`BPLibraryUtils.setNumberValue` _returnvalue "DiceNum" DiceNum))
  (return _returnvalue_2))

(fn `UserConstructionScript`)