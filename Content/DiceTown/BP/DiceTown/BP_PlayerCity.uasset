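; BP_PlayerCity is a player's city in DiceTown, holding that player's index, money and buildings.
; Init stores the index and game mode, then grants starting money and a starter set of buildings.
; On authority, building finds the child of Buildings named row name plus next count and passes its transform to AddBuilding.
; E_Build and FBuild duplicate this logic, and both refresh the UI building list, also on remotes.
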(event `E_Init`
  (params (PlayerIndex :type Integer))
  ;[1 1 1] Event:Init
  ;;[1 1 1] PlayerIndex
  (`self.setPlayerIndex` PlayerIndex)
  ;;[1 1 1] GameMode
  (set `self.BPMainGameMode` (cast `/Game/DiceTown/BP/MainGameSystem/BP_MainGameMode` (`GameplayStatics.GetGameMode`) :!pure true))
  ;;[1 1 1] Init
  (`self.F_Build` 1)
  (`self.F_Build` 3)
  (`self.F_Build` 4)
  (`self.F_Build` 4)
  (`self.F_Build` 4)
  (`self.F_Build` 4)
  (`self.setMoney` 3))

(event `E_Build`
  (params (BuildingId :type Integer))
  ;[1 1 1] Event：建造建筑
  (`/Engine/EditorBlueprintResources/ActorMacros.Switch Has Authority`
    (:`Authority`
      (bind _returnvalue (`self.getBuildingCount` BuildingId))
      (bind _returnvalue_2 (`Building.getBuildingRowName` BuildingId))
      (for _array_element (`SceneComponent.GetChildrenComponents` (`self.Buildings`) false)
        (if (`KismetStringLibrary.EqualEqual_StrStr` (`KismetSystemLibrary.GetObjectName` _array_element) (`KismetStringLibrary.Concat_StrStr` _returnvalue_2 (`KismetStringLibrary.Conv_IntToString` (+ _returnvalue 1))))
          (`self.addBuilding` _returnvalue_2 (`SceneComponent.K2_GetComponentLocation` _array_element) (`SceneComponent.K2_GetComponentRotation` _array_element))
          (break))))
    (:`Remote`
      _))
  (`self.E_ResetUIBuildingList`))

(event `E_ResetUIBuildingList`
  ;[1 1 1] Event：刷新UI建筑列表
  (bind _returnvalue (`self.getUIBuildingList`))
  (set `self.currentUIBuildingList` _returnvalue))

(fn `F_Build`
  (params (BuildingId :type Integer))
  (`/Engine/EditorBlueprintResources/ActorMacros.Switch Has Authority`
    (:`Authority`
      (bind _returnvalue (`self.getBuildingCount` BuildingId))
      (bind _returnvalue_2 (`Building.getBuildingRowName` BuildingId))
      (for _array_element (`SceneComponent.GetChildrenComponents` (`self.Buildings`) false)
        (if (`KismetStringLibrary.EqualEqual_StrStr` (`KismetSystemLibrary.GetObjectName` _array_element) (`KismetStringLibrary.Concat_StrStr` _returnvalue_2 (`KismetStringLibrary.Conv_IntToString` (+ _returnvalue 1))))
          (`self.addBuilding` _returnvalue_2 (`SceneComponent.K2_GetComponentLocation` _array_element) (`SceneComponent.K2_GetComponentRotation` _array_element))
          (break))))
    (:`Remote`
      _))
  (`self.E_ResetUIBuildingList`))

(fn `UserConstructionScript`)